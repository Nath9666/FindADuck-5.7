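; Countdown timer Blueprint that fails the level when time runs out by opening the FinishFail level.
; Each Tick calls the Culdawn event, which subtracts world delta seconds from CountDown, clamps it at zero and shows it as a time string on a TextRender.
; When the next decrement would reach zero, it waits briefly through a Delay before loading that level.
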(event Custom|Culdawn
  (bind _output_get (Variables|Default|SetCountDown (Math|Float|Clamp(Float) (- (Variables|Default|GetCountDown) (Utilities|Time|GetWorldDeltaSeconds)) 0.0 (Variables|Default|GetCountDown))))
  (Utilities|FlowControl|Sequence
    (:then_0
      (Rendering|Components|TextRender|SetText (Variables|Default|GetTextRender) (Utilities|Text|ToText(String) (Class|KismetStringLibrary|TimeSecondstoString _output_get))))
    (:then_1
      (if (== (Math|Float|Clamp(Float) (- (Variables|Default|GetCountDown) (Utilities|Time|GetWorldDeltaSeconds)) 0.0 (Variables|Default|GetCountDown)) 0.0)
        (Utilities|FlowControl|Delay 0.2)
        (Game|OpenLevel(byName) "FinishFail")))))

(event EventBeginPlay)

(event EventTick
  (params (DeltaSeconds :type Float%20%28single-precision%29))
  (CallFunction|Culdawn))

(fn ConstructionScript)